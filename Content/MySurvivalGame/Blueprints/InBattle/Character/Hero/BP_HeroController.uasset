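; BP_HeroController is a hero controller for battle that relays commander tasks to the hero's AI Blackboard.
; SetCommanderTaskBegin sets an executing flag and the task type, then switches on that type to write the target location for move-to-position orders.
; SetCommanderTaskEnd clears the executing flag, and the controller itself contains no movement or tick logic.
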(event Custom|SetCommanderTaskBegin
  (params (CommanderTaskType :type Enum_CommanderTaskType%20Enum) (MoveToPosition :type Vector))
  (bind _blackboard (Variables|Default|GetBlackboard))
  ;[1 1 1] Commander Task
  (AI|Components|Blackboard|SetValueasBool _blackboard (Utilities|Name|MakeLiteralName "IsExcutingCommanderTask") true)
  (AI|Components|Blackboard|SetValueasEnum _blackboard (Utilities|Name|MakeLiteralName "CommanderTaskType") CommanderTaskType)
  (switch Utilities|FlowControl|Switch|SwitchonEnum_CommanderTaskType CommanderTaskType
    (:NewEnumerator0
      ;;[1 1 1] Move To Position Task
      (AI|Components|Blackboard|SetValueasVector (Variables|Default|GetBlackboard) (Utilities|Name|MakeLiteralName "CommanderTargetLocation") MoveToPosition))))

(event Custom|SetCommanderTaskEnd
  ;[1 1 1] Commander Task
  (AI|Components|Blackboard|SetValueasBool (Variables|Default|GetBlackboard) (Utilities|Name|MakeLiteralName "IsExcutingCommanderTask") false))

(event EventBeginPlay
  (|CallParentFunction))

(event EventTick
  (params (DeltaSeconds :type Float%20%28single-precision%29)))

(fn ConstructionScript
  (|CallParentFunction))