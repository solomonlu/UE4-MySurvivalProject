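; BP_AssaultRifleProjectile is the hero's assault rifle projectile, which damages NPCs on contact.
; When its sphere overlaps the capsule of a living BP_NPC_Base that carries the target tag, it applies fixed damage and destroys itself.
; Any blocking hit on the sphere also destroys it, without dealing damage.
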(event OnComponentHit(Sphere)
  (params (HitComponent :type Primitive%20Component%20Object%20Reference) (OtherActor :type Actor%20Object%20Reference) (OtherComp :type Primitive%20Component%20Object%20Reference) (NormalImpulse :type Vector :default "0, 0, 0") (Hit :type Hit%20Result%20Structure%20%28by%20ref%29))
  (Actor|DestroyActor))

(event OnComponentBeginOverlap(Sphere)
  (params (OverlappedComponent :type Primitive%20Component%20Object%20Reference) (OtherActor :type Actor%20Object%20Reference) (OtherComp :type Primitive%20Component%20Object%20Reference) (OtherBodyIndex :type Integer) (bFromSweep :type Boolean) (SweepResult :type Hit%20Result%20Structure%20%28by%20ref%29))
  (bind _asbp_npc_base (Utilities|Casting|CastToBP_NPC_Base OtherActor))
  (if (== OtherComp (Variables|/Script/Engine.Character|GetCapsuleComponent _asbp_npc_base))
    (if (Variables|/Game/AIBehaviorToolkit/Blueprints/BP_BehaviorComponent.BP_BehaviorComponent_C|GetIsAlive (Variables|/Game/AIBehaviorToolkit/Blueprints/BP_NPC_Base.BP_NPC_Base_C|GetBehaviorComponent _asbp_npc_base))
      (if (Actor|ActorHasTag _asbp_npc_base (Variables|Default|GetTargetTag))
        (Game|Damage|ApplyDamage _asbp_npc_base 1e+01 0 0)
        (Actor|DestroyActor)))))

(fn ConstructionScript)