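; Player controller for the battle commander that creates the hero selection HUD and handles the SetDestination input.
; With a hero controlled, holding the input traces under the cursor each frame and sends move tasks to that hero's BP_HeroController, ignoring points too close to the hero.
; Otherwise, dragging moves the commander pawn from its press-time position by the scaled mouse delta, with a cosine factor on one axis.
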(event EventBeginPlay
  ;[1 1 1] create the HUD
  (bind _returnvalue (UserInterface|CreateWidget "/Game/MySurvivalGame/Blueprints/InBattle/UI/UI_HeroesSelectBox.UI_HeroesSelectBox_C" self))
  (UserInterface|Viewport|AddtoViewport _returnvalue 0))

(event EventTick
  (params (DeltaSeconds :type Float%20%28single-precision%29))
  (bind (_locationx _locationy) (Game|Player|GetMousePosition))
  (bind _touchstartmouseposition (Variables|Default|GetTouchStartMousePosition))
  (bind _returnvalue (- _touchstartmouseposition (Math|Vector|MakeVector _locationx _locationy 0.0)))
  (Utilities|FlowControl|Sequence
    (:then_0
      (Utilities|IsValid (Variables|Hero|GetControlledHero)
        (:Is%20Valid
          ;[1 1 1] if controlling a hero, click to tell him go there
          (Utilities|FlowControl|Gate true ; While key is pressed...
            (:Exit
              (CallFunction|MoveControlledHerotoHitLocation (.HitResult (Game|Player|GetHitResultUnderCursorbyChannel "TraceTypeQuery3" true))) ; ..and move there.
            )))
        (:Is%20Not%20Valid
          ;[1 1 1] if not controlling a hero, drag to move commander
          (Utilities|FlowControl|Gate true ; While key is pressed...
            (:Exit
              (Transformation|SetActorLocation (Pawn|GetControlledPawn) (+ (Variables|Default|GetTouchStartCommanderPosition) (* (* (Math|Vector|MakeVector (.y _returnvalue) (* (.x _returnvalue) -1.0 (Math|Trig|Cos(Degrees) 6e+01)) 0.0) -1.0) (Variables|Default|GetMouseMoveScale))) false false))))))))

(event Input|ActionEvents|InputActionSetDestination
  (params (Key :type Key%20Structure :default "AnyKey"))
  (bind (_locationx _locationy) (Game|Player|GetMousePosition))
  (bind (_locationx_2 _locationy_2) (Game|Player|GetMousePosition))
  ;[1 1 1] if not controlling a hero, drag to move commander
  ;;[1 1 1] Record mouse and commander position when touch start
  (:Pressed
    (Variables|Default|SetTouchStartMousePosition (Math|Vector|MakeVector _locationx _locationy 0.0))
    (Variables|Default|SetTouchStartCommanderPosition (Transformation|GetActorLocation (Pawn|GetControlledPawn)))
    (Utilities|FlowControl|Gate true) ; enters at Open
  )
  (:Released
    (Utilities|FlowControl|Gate true) ; enters at Close
  ))

(event Input|ActionEvents|InputActionSetDestination
  (params (Key :type Key%20Structure :default "AnyKey"))
  ;[1 1 1] if controlling a hero, click to tell him go there
  (:Pressed
    (Utilities|FlowControl|Gate true) ; enters at Open
  )
  (:Released
    (Utilities|FlowControl|Gate true) ; enters at Close
  ))

(fn ConstructionScript)

(fn MoveControlledHerotoHitLocation
  (params (Hit :type Hit%20Result%20Structure))
  (bind _location (Collision|BreakHitResult Hit))
  (if (>= (Math|Vector|VectorLength (- (Transformation|GetActorLocation (Variables|Hero|GetControlledHero)) _location)) (Variables|Default|GetMinMoveDistance)) ; Don't move if player clicks too close to pawn
    (bind _asbp_hero_controller (Utilities|Casting|CastToBP_HeroController (Pawn|GetController (Variables|Hero|GetControlledHero))))
    (Default|SetCommanderTaskBegin _asbp_hero_controller "NewEnumerator0" _location)))