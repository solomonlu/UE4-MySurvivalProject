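; BP_CommanderController is the player controller through which the player commands a controlled hero by clicking in the world.
; On BeginPlay it adds the hero selection box widget to the viewport.
; While SetDestination is held, a Tick-driven gate traces under the cursor each frame.
; Hit points at least a minimum distance from the hero go to its BP_HeroController as a commander task with that move position.
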(event EventBeginPlay
  ;[1 1 1] create the HUD
  (bind _returnvalue (UserInterface|CreateWidget "/Game/MySurvivalGame/Blueprints/InBattle/UI/UI_HeroesSelectBox.UI_HeroesSelectBox_C" self))
  (UserInterface|Viewport|AddtoViewport _returnvalue 0))

(event EventTick
  (params (DeltaSeconds :type Float%20%28single-precision%29))
  (Utilities|FlowControl|Sequence
    (:then_0
      (Utilities|IsValid (Variables|Hero|GetControlledHero)
        (:Is%20Valid
          ;[1 1 1] if controlling a hero, click to tell him go there
          (Utilities|FlowControl|Gate true ; While key is pressed...
            (:Exit
              (CallFunction|MoveControlledHerotoHitLocation (.HitResult (Game|Player|GetHitResultUnderCursorbyChannel "TraceTypeQuery1" true))) ; ..and move there.
            )))))))

(event Input|ActionEvents|InputActionSetDestination
  (params (Key :type Key%20Structure :default "AnyKey"))
  ;[1 1 1] if controlling a hero, click to tell him go there
  (:Pressed
    (Utilities|FlowControl|Gate true) ; enters at Open
  )
  (:Released
    (Utilities|FlowControl|Gate true) ; enters at Close
  ))

(fn ConstructionScript)

(fn MoveControlledHerotoHitLocation
  (params (Hit :type Hit%20Result%20Structure))
  (bind _location (Collision|BreakHitResult Hit))
  (if (>= (Math|Vector|VectorLength (- (Transformation|GetActorLocation (Variables|Hero|GetControlledHero)) _location)) (Variables|Default|GetMinMoveDistance)) ; Don't move if player clicks too close to pawn
    (Default|SetCommanderTaskBegin (.AsBP%20Hero%20Controller (Utilities|Casting|CastToBP_HeroController (Pawn|GetController (Variables|Hero|GetControlledHero)))) "NewEnumerator0" _location)))